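; BP_FinalDoor is a double wooden door that the player can open only after taking the key.
; Its Interaction event reads KeyTaken on the first-person player character and plays a 2D lock-fail sound if the key is missing.
; With the key, it plays an opening sound at the doorway and runs a timeline that yaws the two leaves in opposite directions, mirroring one track by negation.
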(event `/Game/BPI/BPI_Interaction.Interaction`
  (bind _asbp_first_person_character (cast `/Game/FirstPerson/Blueprints/BP_FirstPersonCharacter` (`GameplayStatics.GetPlayerCharacter` 0)))
  (if (`/Game/FirstPerson/Blueprints/BP_FirstPersonCharacter.Key_Taken` _asbp_first_person_character)
    (`GameplayStatics.PlaySoundAtLocation` "/Game/Sound/Cues/SC_OpenWoodenDoor.SC_OpenWoodenDoor" (`SceneComponent.K2_GetComponentLocation` (`self.SM_DoorWay`)) (struct) 1.0 1.0 0.0 null null null null)
    (bind (_direction _newtrack_0) (`Timeline|Timeline` :!via `PlayFromStart`)
      (:`Update`
        (`SceneComponent.K2_SetRelativeRotation` (`self.SM_DoorWay_Large_Door_Right`) (`KismetMathLibrary.MakeRotator` 0.0 0.0 _newtrack_0) false false)
        (`SceneComponent.K2_SetRelativeRotation` (`self.SM_DoorWay_Large_Door_Left`) (`KismetMathLibrary.MakeRotator` 0.0 0.0 (* _newtrack_0 -1.0)) false false)))
    (else
      (`GameplayStatics.PlaySound2D` "/Game/Sound/Cues/SC_TryLockFail.SC_TryLockFail" 1.0 1.0 0.0 null null))))

(fn `UserConstructionScript`)