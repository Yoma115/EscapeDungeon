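; BP_Cell_Door is a metal cell door that toggles open and closed through its Interaction event.
; Each interaction plays the metal door sound at the mesh location and flips the IsOpen flag.
; The TL_OpenDoor timeline plays from start to open or reverses from end to close, driving the SMCellDoor mesh's relative yaw.
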(event `self.ReceiveBeginPlay`)

(event `/Game/BPI/BPI_Interaction.Interaction`
  (`GameplayStatics.PlaySoundAtLocation` "/Game/Sound/Cues/SC_OpenMetalDoor.SC_OpenMetalDoor" (`SceneComponent.K2_GetComponentLocation` (`self.SM_Cell_Door`)) (struct) 1.0 1.0 0.0 null null null null)
  (if (`self.IsOpen`)
    (set `self.IsOpen` false)
    (bind (_direction _newtrack_0) (`Timeline|TL_OpenDoor` :!via `ReverseFromEnd` :!label _label)
      (:`Update`
        (`SceneComponent.K2_SetRelativeRotation` (`self.SM_Cell_Door`) (`KismetMathLibrary.MakeRotator` 0.0 0.0 _newtrack_0) false false)))
    (else
      (set `self.IsOpen` true)
      (goto _label :!via `PlayFromStart`))))

(fn `UserConstructionScript`)